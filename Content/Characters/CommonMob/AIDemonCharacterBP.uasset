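; Common mob demon enemy character that walks, runs, attacks with either hand and can be killed.
; Speeds, max health and attack damage come from the CommonMob row of Enemy_DataTable.
; Attack animations open a timed window where socket-attached hand colliders damage NoSwordBP on overlap.
; Incoming hits trigger brief invulnerability; death stops AI logic, ragdolls the mesh and destroys the actor after a delay.
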(event OnComponentBeginOverlap(LeftHand)
  (params (OverlappedComponent :type Primitive%20Component%20Object%20Reference) (OtherActor :type Actor%20Object%20Reference) (OtherComp :type Primitive%20Component%20Object%20Reference) (OtherBodyIndex :type Integer) (bFromSweep :type Boolean) (SweepResult :type Hit%20Result%20Structure%20%28by%20ref%29))
  ;[1 1 1] Doing Damage
  (if (Variables|Default|GetAttacking)
    (bind _asno_sword_bp (Utilities|Casting|CastToNoSwordBP OtherActor))
    (bind _returnvalue (Utilities|GetDataTableRow "/Game/Core/Enemy_DataTable.Enemy_DataTable" "CommonMob")
      (:then
        (Default|TakeDamage _asno_sword_bp (.Attack_Damage (Utilities|Struct|BreakEnemy_Data_Struct _returnvalue)))))))

(event OnComponentBeginOverlap(RightHand)
  (params (OverlappedComponent :type Primitive%20Component%20Object%20Reference) (OtherActor :type Actor%20Object%20Reference) (OtherComp :type Primitive%20Component%20Object%20Reference) (OtherBodyIndex :type Integer) (bFromSweep :type Boolean) (SweepResult :type Hit%20Result%20Structure%20%28by%20ref%29))
  ;[1 1 1] Doing Damage
  (if (Variables|Default|GetAttacking)
    (bind _asno_sword_bp (Utilities|Casting|CastToNoSwordBP OtherActor))
    (bind _returnvalue (Utilities|GetDataTableRow "/Game/Core/Enemy_DataTable.Enemy_DataTable" "CommonMob")
      (:then
        (Default|TakeDamage _asno_sword_bp (.Attack_Damage (Utilities|Struct|BreakEnemy_Data_Struct _returnvalue)))))))

(event Custom|Walk
  ;[1 1 1] Movement
  (Utilities|GetDataTableRow "/Game/Core/Enemy_DataTable.Enemy_DataTable" "CommonMob"
    (:then
      (Variables|/Script/Engine.CharacterMovementComponent|SetMaxWalkSpeed (Variables|Character|GetCharacterMovement) (.Walk_Speed (Utilities|Struct|BreakEnemy_Data_Struct (stale Custom|Run _returnvalue)))))))

(event Custom|AttackRight
  ;[1 1 1] Attacking
  (Components|Animation|PlayAnimation (Variables|Character|GetMesh) "/Game/Characters/CommonMob/Animations/Demon_Attack_Right.Demon_Attack_Right" false)
  (Utilities|FlowControl|Delay 0.883)
  (Variables|Default|SetAttacking true)
  (Utilities|FlowControl|Delay 0.363)
  (Variables|Default|SetAttacking false)
  (Utilities|FlowControl|Delay 1.387)
  (Components|Animation|SetAnimationMode (Variables|Character|GetMesh) "AnimationBlueprint"))

(event Custom|DemonTakeDamage
  (params (DemonIncomingDamage :type Integer))
  ;[1 1 1] Taking Damage
  (if (Variables|Default|GetDemonCanBeHit)
    (Audio|PlaySoundatLocation "/Game/Characters/CommonMob/Sounds/Enemy_Hit.Enemy_Hit" (Transformation|GetActorLocation self))
    (bind _output_get (Variables|Default|SetDemonHealth (- (Variables|Default|GetDemonHealth) DemonIncomingDamage)))
    (bind _output_get_2 (Variables|Default|SetIsDead (<= _output_get 0)))
    (if _output_get_2
      (Variables|Default|SetDemonCanBeHit false)
      (Variables|Default|SetAttacking false)
      (AI|Logic|StopLogic (Variables|/Script/AIModule.AIController|GetBrainComponent (AI|GetAIController self)) "")
      (Components|Movement|StopMovementImmediately (Variables|Character|GetCharacterMovement))
      (Utilities|FlowControl|DoOnce false
        (:Completed
          (Audio|SpawnSoundatLocation "/Game/Characters/CommonMob/Sounds/OOT_Stalchild_DieX.OOT_Stalchild_DieX" (Transformation|GetActorLocation self))
          (Physics|SetSimulatePhysics (Variables|Character|GetMesh) true)
          (Utilities|FlowControl|Delay 4.0)
          (Actor|DestroyActor)))
      (else
        (Variables|Default|SetDemonCanBeHit false)
        (Utilities|FlowControl|Delay 1.0)
        (Variables|Default|SetDemonCanBeHit true)))))

(event Custom|AttackLeft
  ;[1 1 1] Attacking
  (Components|Animation|PlayAnimation (Variables|Character|GetMesh) "/Game/Characters/CommonMob/Animations/Demon_Attack_Left.Demon_Attack_Left" false)
  (Utilities|FlowControl|Delay 0.883)
  (Variables|Default|SetAttacking true)
  (Utilities|FlowControl|Delay 0.363)
  (Variables|Default|SetAttacking false)
  (Utilities|FlowControl|Delay 1.387)
  (Components|Animation|SetAnimationMode (Variables|Character|GetMesh) "AnimationBlueprint"))

(event Custom|Run
  ;[1 1 1] Movement
  (bind _returnvalue (Utilities|GetDataTableRow "/Game/Core/Enemy_DataTable.Enemy_DataTable" "CommonMob")
    (:then
      (Variables|/Script/Engine.CharacterMovementComponent|SetMaxWalkSpeed (Variables|Character|GetCharacterMovement) (.Run_Speed (Utilities|Struct|BreakEnemy_Data_Struct _returnvalue))))))

(fn ConstructionScript
  (bind _returnvalue (Utilities|GetDataTableRow "/Game/Core/Enemy_DataTable.Enemy_DataTable" "CommonMob")
    (:then
      (Variables|Default|SetDemonHealth (.Max_Health (Utilities|Struct|BreakEnemy_Data_Struct _returnvalue)))
      (Transformation|AttachComponentToComponent (Variables|Default|GetRightHand) (Variables|Character|GetMesh) "RightHandSocket" "KeepRelative" "KeepRelative" "KeepRelative" true)
      (Transformation|AttachComponentToComponent (Variables|Default|GetLeftHand) (Variables|Character|GetMesh) "LeftHandSocket" "KeepRelative" "KeepRelative" "KeepRelative" true))))