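; Titan boss character that, once initialized, shows a health bar and chases the player.
; A looping distance timer triggers random melee montages up close or occasional ranged montages farther away, pausing the recursive AIMoveTo seek during attacks.
; Events toggle fist collision and sphere-trace from the fists to spawn hit particles on the player.
; Attacks set damage ranges, but nothing here applies damage and fist overlaps are stubs.
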(event OnComponentBeginOverlap(RightFist)
  (params (OverlappedComponent :type Primitive%20Component%20Object%20Reference) (OtherActor :type Actor%20Object%20Reference) (OtherComp :type Primitive%20Component%20Object%20Reference) (OtherBodyIndex :type Integer) (bFromSweep :type Boolean) (SweepResult :type Hit%20Result%20Structure%20%28by%20ref%29))
  (if (== OtherActor (Game|GetPlayerCharacter 0))
    _))

(event OnComponentBeginOverlap(LeftFist)
  (params (OverlappedComponent :type Primitive%20Component%20Object%20Reference) (OtherActor :type Actor%20Object%20Reference) (OtherComp :type Primitive%20Component%20Object%20Reference) (OtherBodyIndex :type Integer) (bFromSweep :type Boolean) (SweepResult :type Hit%20Result%20Structure%20%28by%20ref%29))
  (if (== (Game|GetPlayerCharacter 0) OtherActor)
    _))

(event Custom|Seek%20Player
  ;[1 1 1] Seeking Player Loop
  (if (Variables|Default|GetisAttacking)
    (Components|Movement|StopMovementImmediately (Variables|Character|GetCharacterMovement))
    (else
      (AI|AIMoveTo self "0, 0, 0" (Game|GetPlayerCharacter 0) 1.5e+02 false
        (:then
          _)
        (:OnSuccess
          _)
        (:OnFail
          _))
      (Utilities|FlowControl|Delay 0.2)
      (CallFunction|SeekPlayer))))

(event Custom|RightFistCollisionEnable
  ;[1 1 1] Fist Collision Enable/Disable
  (Collision|SetCollisionEnabled (Variables|Default|GetRightFist) "QueryAndPhysics"))

(event Custom|FacePlayer
  ;[1 1 1] Face Player
  (Transformation|SetActorRotation (Math|Rotator|MakeRotator 0.0 0.0 (.Yaw (Math|Rotator|BreakRotator (Math|Rotator|FindLookatRotation (Transformation|GetActorLocation) (Transformation|GetActorLocation (Game|GetPlayerCharacter 0))))))))

(event Custom|RightFistCollisionDisable
  ;[1 1 1] Fist Collision Enable/Disable
  (Collision|SetCollisionEnabled (Variables|Default|GetRightFist) "NoCollision"))

(event Custom|InitTitanBoss
  ;[1 1 1] Initialize Boss
  (Variables|Default|SetAlive true)
  (Variables|Default|SetHealth 1e+03)
  (bind _returnvalue (UserInterface|CreateWidget "/Game/Core/BossHealthBar.BossHealthBar_C"))
  (UserInterface|Viewport|AddtoViewport _returnvalue 0)
  (Utilities|FlowControl|Delay 0.2)
  (CallFunction|SeekPlayer)
  (CallFunction|FindPlayerDistance))

(event Custom|LeftFistCollisionDisable
  ;[1 1 1] Fist Collision Enable/Disable
  (Collision|SetCollisionEnabled (Variables|Default|GetLeftFist) "NoCollision"))

(event Custom|FindPlayerDistance
  ;[1 1 1] Get Player Distance (Function Call)
  (Utilities|Time|SetTimerbyFunctionName 0 "PlayerDistance" 1.5 true))

(event Custom|L_Trace
  (bind _leftfist (Variables|Default|GetLeftFist))
  (bind _returnvalue (Transformation|GetWorldLocation _leftfist))
  (bind _returnvalue_2 (Transformation|GetWorldRotation _leftfist))
  (bind _returnvalue_3 (Math|Vector|GetForwardVector _returnvalue_2))
  (bind _returnvalue_4 (+ _returnvalue _returnvalue_3))
  (bind _outhit (Collision|SphereTraceForObjects _returnvalue_4 _returnvalue_4 1e+03 (Utilities|Array|MakeArray "ObjectTypeQuery3") false 0 "None"))
  (if (== (.HitActor (Collision|BreakHitResult _outhit)) (Game|GetPlayerCharacter 0))
    (Effects|SpawnEmitteratLocation "/Game/StarterContent/Particles/P_FistSprite.P_FistSprite" (.Location (Collision|BreakHitResult _outhit)))))

(event Custom|R_Trace
  (bind _rightfist (Variables|Default|GetRightFist))
  (bind _returnvalue (Transformation|GetWorldLocation _rightfist))
  (bind _returnvalue_2 (Transformation|GetWorldRotation _rightfist))
  (bind _returnvalue_3 (Math|Vector|GetForwardVector _returnvalue_2))
  (bind _returnvalue_4 (+ _returnvalue _returnvalue_3))
  (bind _outhit (Collision|SphereTraceForObjects _returnvalue_4 _returnvalue_4 1e+03 (Utilities|Array|MakeArray "ObjectTypeQuery3") false 0 "None"))
  (if (== (.HitActor (Collision|BreakHitResult _outhit)) (Game|GetPlayerCharacter 0))
    (Effects|SpawnEmitteratLocation "/Game/StarterContent/Particles/P_FistSprite.P_FistSprite" (.Location (Collision|BreakHitResult _outhit)))))

(event Custom|LongRange
  ;[1 1 1] Attack Picker
  (Variables|Default|SetisAttacking true)
  (switch int (Math|Random|RandomIntegerinRange 0 1)
    (:0
      (Variables|Default|SetAttMontage "/Game/Characters/TitanBoss/Animations/TitanRange01.TitanRange01")
      (Variables|Default|SetMinDamage 2e+01)
      (Variables|Default|SetMaxDamage 23.0))
    (:1
      (Variables|Default|SetAttMontage "/Game/Characters/TitanBoss/Animations/TitanRange02.TitanRange02")
      (Variables|Default|SetMinDamage 0.0)
      (Variables|Default|SetMaxDamage 0.0)))
  (bind _returnvalue (Animation|PlayAnimMontage (Variables|Default|GetAttMontage) 1.0 "None"))
  (Utilities|FlowControl|Delay _returnvalue)
  (Variables|Default|SetisAttacking false)
  (CallFunction|SeekPlayer)
  (if (not (>= (Variables|Default|GetDistance) 3e+02))
    (CallFunction|FacePlayer)))

(event Custom|LeftFistCollisionEnable
  ;[1 1 1] Fist Collision Enable/Disable
  (Collision|SetCollisionEnabled (Variables|Default|GetLeftFist) "QueryAndPhysics"))

(event Custom|CloseRange
  ;[1 1 1] Attack Picker
  (Variables|Default|SetisAttacking true)
  (switch int (Math|Random|RandomIntegerinRange 0 2)
    (:0
      (Variables|Default|SetAttMontage "/Game/Characters/TitanBoss/Animations/TitanMelee01.TitanMelee01")
      (Variables|Default|SetMinDamage 1e+01)
      (Variables|Default|SetMaxDamage 15.0))
    (:1
      (Variables|Default|SetAttMontage "/Game/Characters/TitanBoss/Animations/TitanMelee02.TitanMelee02")
      (Variables|Default|SetMinDamage 1e+01)
      (Variables|Default|SetMaxDamage 12.0))
    (:2
      (Variables|Default|SetAttMontage "/Game/Characters/TitanBoss/Animations/TitanMelee03.TitanMelee03")
      (Variables|Default|SetMinDamage 15.0)
      (Variables|Default|SetMaxDamage 2e+01)))
  (bind _returnvalue (Animation|PlayAnimMontage (Variables|Default|GetAttMontage) 1.0 "None"))
  (Utilities|FlowControl|Delay _returnvalue)
  (Variables|Default|SetisAttacking false)
  (CallFunction|SeekPlayer)
  (if (not (>= (Variables|Default|GetDistance) 3e+02))
    (CallFunction|FacePlayer)))

(fn ConstructionScript)

(fn PlayerDistance
  (if (not (Variables|Default|GetisAttacking))
    (bind _output_get (Variables|Default|SetDistance (Math|Vector|VectorLength (- (Transformation|GetActorLocation) (Transformation|GetActorLocation (Game|GetPlayerCharacter 0))))))
    (if (>= _output_get 3e+02)
      (if (== (Math|Random|RandomIntegerinRange 0 6) 0)
        (CallFunction|LongRange)
        (else
          (CallFunction|SeekPlayer)))
      (else
        (CallFunction|CloseRange)))))