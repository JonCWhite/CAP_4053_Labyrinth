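; Fireball projectile actor for the Titan boss that bursts when it touches the NoSwordBP character.
; Its sphere turns on collision shortly after spawn, and the actor destroys itself after a few seconds if nothing is hit.
; An overlap with that exact class, gated by a cast of the player character, spawns a hit particle and destroys the fireball a moment later.
; No damage is applied in this graph.
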(event OnComponentBeginOverlap(Sphere)
  (params (OverlappedComponent :type Primitive%20Component%20Object%20Reference) (OtherActor :type Actor%20Object%20Reference) (OtherComp :type Primitive%20Component%20Object%20Reference) (OtherBodyIndex :type Integer) (bFromSweep :type Boolean) (SweepResult :type Hit%20Result%20Structure%20%28by%20ref%29))
  (if (== (Utilities|GetClass OtherActor) "/Game/Characters/NoSword/NoSwordBP.NoSwordBP_C")
    (Utilities|Casting|CastToNoSwordBP (Game|GetPlayerCharacter 0))
    (Effects|SpawnEmitteratLocation "/Game/StarterContent/Particles/P_FireballHit.P_FireballHit" (Transformation|GetWorldLocation (Variables|Default|GetSphere)))
    (Utilities|FlowControl|Delay 0.05)
    (Actor|DestroyActor)))

(event EventBeginPlay
  (Utilities|FlowControl|Delay 0.2)
  (Collision|SetCollisionEnabled (Variables|Default|GetSphere) "QueryAndPhysics")
  (Utilities|FlowControl|Delay 7.5)
  (Actor|DestroyActor))

(event Collision|EventActorBeginOverlap
  (params (OtherActor :type Actor%20Object%20Reference)))

(event EventTick
  (params (DeltaSeconds :type Float%20%28single-precision%29)))

(fn ConstructionScript)