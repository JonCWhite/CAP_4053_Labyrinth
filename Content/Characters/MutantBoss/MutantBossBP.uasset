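; Mutant boss enemy that chases the player and picks melee or ranged attacks by distance.
; InitMutantBoss sets health, shows a health bar widget, then starts a recursive AIMoveTo seek loop and a looping distance timer.
; While idle, the timer triggers random close-range montages when near, or occasional long-range ones when far.
; Attacks block re-triggering until the montage ends, then resume seeking and snap yaw toward a nearby player.
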(event Custom|Seek%20Player
  ;[1 1 1] Seeking Player Loop
  (if (Variables|Default|GetisAttacking)
    (Components|Movement|StopMovementImmediately (Variables|Character|GetCharacterMovement))
    (else
      (AI|AIMoveTo self "0, 0, 0" (Game|GetPlayerCharacter 0) 1.5e+02 false
        (:then
          _)
        (:OnSuccess
          _)
        (:OnFail
          _))
      (Utilities|FlowControl|Delay 0.2)
      (CallFunction|SeekPlayer))))

(event Custom|FacePlayer
  ;[1 1 1] Face Player
  (Transformation|SetActorRotation (Math|Rotator|MakeRotator 0.0 0.0 (.Yaw (Math|Rotator|BreakRotator (Math|Rotator|FindLookatRotation (Transformation|GetActorLocation) (Transformation|GetActorLocation (Game|GetPlayerCharacter 0))))))))

(event Custom|InitMutantBoss
  ;[1 1 1] Initialize Boss
  (Variables|Default|SetAlive true)
  (Variables|Default|SetHealth 1e+03)
  (bind _returnvalue (UserInterface|CreateWidget "/Game/Core/BossHealthBar.BossHealthBar_C"))
  (UserInterface|Viewport|AddtoViewport _returnvalue 0)
  (Utilities|FlowControl|Delay 0.2)
  (CallFunction|SeekPlayer)
  (CallFunction|FindPlayerDistance))

(event Custom|FindPlayerDistance
  ;[1 1 1] Get Player Distance (Function Call)
  (Utilities|Time|SetTimerbyFunctionName 0 "PlayerDistance" 1.0 true))

(event Custom|LongRange
  ;[1 1 1] Attack Picker
  (Variables|Default|SetisAttacking true)
  (switch int (Math|Random|RandomIntegerinRange 0 1)
    (:0
      (Variables|Default|SetAttMontage "/Game/Characters/MutantBoss/Animations/MutantRange01.MutantRange01"))
    (:1
      (Variables|Default|SetAttMontage "/Game/Characters/MutantBoss/Animations/MutantRange02.MutantRange02")))
  (bind _returnvalue (Animation|PlayAnimMontage (Variables|Default|GetAttMontage) 1.0 "None"))
  (Utilities|FlowControl|Delay _returnvalue)
  (Variables|Default|SetisAttacking false)
  (CallFunction|SeekPlayer)
  (if (not (>= (Variables|Default|GetDistance) 3e+02))
    (CallFunction|FacePlayer)))

(event Custom|CloseRange
  ;[1 1 1] Attack Picker
  (Variables|Default|SetisAttacking true)
  (switch int (Math|Random|RandomIntegerinRange 0 2)
    (:0
      (Variables|Default|SetAttMontage "/Game/Characters/MutantBoss/Animations/MutantClose01.MutantClose01"))
    (:1
      (Variables|Default|SetAttMontage "/Game/Characters/MutantBoss/Animations/MutantClose02.MutantClose02"))
    (:2
      (Variables|Default|SetAttMontage "/Game/Characters/MutantBoss/Animations/MutantClose03.MutantClose03")))
  (bind _returnvalue (Animation|PlayAnimMontage (Variables|Default|GetAttMontage) 1.0 "None"))
  (Utilities|FlowControl|Delay _returnvalue)
  (Variables|Default|SetisAttacking false)
  (CallFunction|SeekPlayer)
  (if (not (>= (Variables|Default|GetDistance) 3e+02))
    (CallFunction|FacePlayer)))

(fn ConstructionScript)

(fn PlayerDistance
  (if (not (Variables|Default|GetisAttacking))
    (bind _output_get (Variables|Default|SetDistance (Math|Vector|VectorLength (- (Transformation|GetActorLocation) (Transformation|GetActorLocation (Game|GetPlayerCharacter 0))))))
    (if (>= _output_get 3e+02)
      (if (== (Math|Random|RandomIntegerinRange 0 6) 0)
        (CallFunction|LongRange)
        (else
          (CallFunction|SeekPlayer)))
      (else
        (CallFunction|CloseRange)))))