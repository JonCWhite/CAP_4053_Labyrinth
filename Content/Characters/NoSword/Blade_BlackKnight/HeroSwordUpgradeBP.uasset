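; HeroSwordUpgradeBP is the hero's upgraded sword, which damages demon and Titan boss enemies it overlaps.
; On overlap it casts the player character to NoSwordBP and deals damage only while that character's CanDoDamage flag is set.
; An exact class check routes SwordDamage to DemonTakeDamage on AIDemonCharacterBP or TitanTakeDamage on TitanBossBP, ignoring all other actors, including subclasses.
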(event Collision|EventActorBeginOverlap
  (params (OtherActor :type Actor%20Object%20Reference))
  ;[1 1 1] Hit Detection
  (bind _asno_sword_bp (Utilities|Casting|CastToNoSwordBP (Game|GetPlayerCharacter 0)))
  (if (Variables|/Game/Characters/NoSword/NoSwordBP.NoSwordBP_C|GetCanDoDamage _asno_sword_bp)
    (if (== (Utilities|GetClass OtherActor) "/Game/Characters/CommonMob/AIDemonCharacterBP.AIDemonCharacterBP_C")
      (bind _asaidemon_character_bp (Utilities|Casting|CastToAIDemonCharacterBP OtherActor))
      (Default|DemonTakeDamage _asaidemon_character_bp (Variables|Default|GetSwordDamage))
      (elif (== (Utilities|GetClass OtherActor) "/Game/Characters/TitanBoss/TitanBossBP.TitanBossBP_C")
        (bind _astitan_boss_bp (Utilities|Casting|CastToTitanBossBP OtherActor))
        (Default|TitanTakeDamage _astitan_boss_bp (Variables|Default|GetSwordDamage))))))

(fn ConstructionScript)